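; Reflection component for the Aximmetry virtual camera setup that renders a supplied texture on a mesh through a Billboard-based dynamic material, created at BeginPlay.
; Its Tick function takes state from the caller, toggles visibility and, while active, applies the world transform, texture and lit, tonemap-bypass and alpha-correction flags.
; Inverse tonemap textures are bound for bypass or alpha correction, with the forward tonemap added only for alpha correction.
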(event EventBeginPlay
  (bind _returnvalue (Rendering|Material|CreateDynamicMaterialInstance 0 "/Game/Aximmetry_VirtualCam_3-Bill/Materials/Shaders/Billboard.Billboard" "None" :!class /Script/Engine.PrimitiveComponent))
  (Variables|Default|SetDynamic%20Material%20Instance _returnvalue))

(fn Tick
  (params (Active :type Boolean) (Lit :type Boolean) (Bypass%20Tonemapper :type Boolean) (Texture :type Texture%20Object%20Reference) (Transform :type Transform) (AlphaCorrection :type Boolean))
  (bind _dynamic_material_instance (Variables|Default|GetDynamic%20Material%20Instance))
  (Rendering|SetVisibility Active false)
  (if Active
    (Transformation|SetWorldTransform Transform false false)
    (Rendering|Material|SetTextureParameterValue (Variables|Default|GetDynamic%20Material%20Instance) "Texture" Texture)
    (Rendering|Material|SetScalarParameterValue (Variables|Default|GetDynamic%20Material%20Instance) "Inverse Tonemap" (Math|Conversions|ToFloat(Boolean) Bypass%20Tonemapper) :!class /Script/Engine.MaterialInstanceDynamic)
    (Rendering|Material|SetScalarParameterValue (Variables|Default|GetDynamic%20Material%20Instance) "Lit" (Math|Conversions|ToFloat(Boolean) Lit) :!class /Script/Engine.MaterialInstanceDynamic)
    (Rendering|Material|SetScalarParameterValue (Variables|Default|GetDynamic%20Material%20Instance) "AlphaCorrection" (Math|Conversions|ToFloat(Boolean) AlphaCorrection) :!class /Script/Engine.MaterialInstanceDynamic)
    (if (or Bypass%20Tonemapper AlphaCorrection)
      (bind (_tonemap _inversetonemap) (Class|AximmetryFunctionLibrary|GetTonemapTextures))
      (Rendering|Material|SetTextureParameterValue _dynamic_material_instance "InverseTonemapTexture" _inversetonemap)
      (if AlphaCorrection
        (Rendering|Material|SetTextureParameterValue _dynamic_material_instance "TonemapTexture" _tonemap)))))