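; Shadow component for an Aximmetry virtual camera billboard, rendering through a dynamic instance of a Shadow material created at BeginPlay.
; Its Tick function sets visibility and, when active, moves the component and feeds textures, depth, lighting and ray tracing settings into the material.
; The shadow texture falls back to the billboard texture without positive depth.
; Bypassing the tonemapper also supplies an inverse tonemap texture.
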(event EventBeginPlay
  (bind _returnvalue (Rendering|Material|CreateDynamicMaterialInstance 0 "/Game/Aximmetry_VirtualCam_3-Bill/Materials/Shaders/Shadow.Shadow" "None" :!class /Script/Engine.PrimitiveComponent))
  (Variables|Default|SetDynamic%20Material%20Instance _returnvalue))

(fn Tick
  (params (Active :type Boolean) (Transform :type Transform) (BillboardTexture :type Texture%20Object%20Reference) (ShadowTexture :type Texture%20Object%20Reference) (RayTraced :type Boolean) (Depth :type Float%20%28double-precision%29) (BypassTonemapper :type Boolean) (Lit :type Boolean) (RayTracedReflectionIntensity :type Float%20%28single-precision%29))
  (Rendering|SetVisibility Active false)
  (if Active
    (Transformation|SetWorldTransform Transform false false)
    (Rendering|Material|SetTextureParameterValue (Variables|Default|GetDynamic%20Material%20Instance) "Texture" BillboardTexture)
    (Rendering|Material|SetScalarParameterValue (Variables|Default|GetDynamic%20Material%20Instance) "Inverse Tonemap" (Math|Conversions|ToFloat(Boolean) BypassTonemapper) :!class /Script/Engine.MaterialInstanceDynamic)
    (Rendering|Material|SetTextureParameterValue (Variables|Default|GetDynamic%20Material%20Instance) "ShadowTexture" (select (> Depth 0.0) ShadowTexture BillboardTexture))
    (Rendering|Material|SetScalarParameterValue (Variables|Default|GetDynamic%20Material%20Instance) "RayTraced" (Math|Conversions|ToFloat(Boolean) RayTraced) :!class /Script/Engine.MaterialInstanceDynamic)
    (Rendering|Material|SetScalarParameterValue (Variables|Default|GetDynamic%20Material%20Instance) "Depth" (* Depth 1e+02) :!class /Script/Engine.MaterialInstanceDynamic)
    (Rendering|Material|SetScalarParameterValue (Variables|Default|GetDynamic%20Material%20Instance) "Lit" (Math|Conversions|ToFloat(Boolean) Lit) :!class /Script/Engine.MaterialInstanceDynamic)
    (if BypassTonemapper
      (bind _inversetonemap (Class|AximmetryFunctionLibrary|GetTonemapTextures))
      (Rendering|Material|SetTextureParameterValue (Variables|Default|GetDynamic%20Material%20Instance) "InverseTonemapTexture" _inversetonemap))
    (Rendering|Material|SetScalarParameterValue (Variables|Default|GetDynamic%20Material%20Instance) "RayTracedReflectionIntensity" RayTracedReflectionIntensity :!class /Script/Engine.MaterialInstanceDynamic)))