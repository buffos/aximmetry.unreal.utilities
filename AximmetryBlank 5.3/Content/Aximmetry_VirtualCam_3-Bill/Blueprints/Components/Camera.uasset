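; Camera component Blueprint for an Aximmetry virtual camera that lets Aximmetry drive the lens and transform.
; BeginPlay switches the player view to a given target actor and removes lens limits so incoming values are not clamped.
; Each Tick applies the supplied field of view, focus distance converted from meters to centimeters, and world transform.
; It also derives filmback sensor width from sensor height and aspect ratio.
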(fn BeginPlay
  (params (View%20Target%20Actor :type Actor%20Object%20Reference))
  (Game|Player|SetViewTargetwithBlend (Game|GetPlayerController 0) View%20Target%20Actor 0.0 "VTBlend_Linear" 0.0 false)
  (Utilities|Struct|SetmembersinCameraLensSettings (Variables|Default|GetLensSettings) 0.0 999999.0 0.0 999999.0 0.0) ; Allow Aximmetry full control over the lens parameters.\n(We don't want Unreal to clamp them to realistic values.)\nNote: Focus Distance = 0 means DOF is disabled.
)

(fn Tick
  (params (Horizontal%20FOV :type Float%20%28double-precision%29) (Focus%20Distance%20In%20Meters :type Float%20%28double-precision%29) (Aspect%20Ratio :type Float%20%28double-precision%29) (Transform :type Transform))
  (Camera|SetFieldOfView Horizontal%20FOV)
  (Utilities|Struct|SetmembersinCameraFocusSettings (Variables|Default|GetFocusSettings) (* Focus%20Distance%20In%20Meters 1e+02))
  (Transformation|SetWorldTransform Transform false false)
  (Variables|Default|SetFilmback (Utilities|Struct|MakeCameraFilmbackSettings (* (.sensorheight (Variables|Default|GetFilmback)) Aspect%20Ratio) (.sensorheight (Variables|Default|GetFilmback)))))