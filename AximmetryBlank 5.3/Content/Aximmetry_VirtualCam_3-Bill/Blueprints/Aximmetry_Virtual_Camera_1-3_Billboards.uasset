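; Aximmetry virtual camera actor that renders three video billboards in Unreal, active while the tracked camera is off.
; Tick reads Aximmetry inputs to drive the camera, HDR output and each billboard's reflection, shadow, depth and AO components.
; Reflection components are chosen from reflection and ray-tracing cvars cached at BeginPlay.
; Per-billboard clip-plane scene captures create light-wrap masks, which MaskMerger packs into RGB for return to Aximmetry.
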(event Custom|OnCameraCut
  (Class|PlayerCameraManager|SetGameCameraCutThisFrame (Game|GetPlayerCameraManager 0))
  (Variables|/Script/Engine.SceneCaptureComponent2D|SetbCameraCutThisFrame (Variables|Default|GetB1%20Light%20Wrap%20Mask%20Capture) true)
  (Variables|/Script/Engine.SceneCaptureComponent2D|SetbCameraCutThisFrame (Variables|Default|GetB2%20Light%20Wrap%20Mask%20Capture) true)
  (Variables|/Script/Engine.SceneCaptureComponent2D|SetbCameraCutThisFrame (Variables|Default|GetB3%20Light%20Wrap%20Mask%20Capture) true))

(event EventBeginPlay
  (|CallParentFunction)
  (Default|BeginPlay (Variables|Default|GetCamera) self)
  (CallFunction|InitializeLightWrapCapture (Variables|Default|GetB1%20Light%20Wrap%20Mask%20Capture))
  (CallFunction|InitializeLightWrapCapture (Variables|Default|GetB2%20Light%20Wrap%20Mask%20Capture))
  (CallFunction|InitializeLightWrapCapture (Variables|Default|GetB3%20Light%20Wrap%20Mask%20Capture))
  (Default|BeginPlay (Variables|Default|GetMask%20Merger))
  (EventDispatchers|AssignTrigger (Class|AximmetryFunctionLibrary|GetAximmetryTrigger "B1 Data:Camera Cut" 122) (delegate Custom|OnCameraCut))
  (bind _returnvalue (Development|GetConsoleVariableIntValue "r.ReflectionMethod"))
  (Variables|Default|SetReflectionMethod _returnvalue)
  (bind _returnvalue_2 (Development|GetConsoleVariableBoolValue "r.RayTracing.Shadows"))
  (Variables|Default|SetRayTracingShadows _returnvalue_2)
  (bind _returnvalue_3 (Development|GetConsoleVariableBoolValue "r.Lumen.HardwareRayTracing"))
  (Variables|Default|SetLumenHardwareRayTracing _returnvalue_3)
  (bind _returnvalue_4 (Development|GetConsoleVariableIntValue "r.Lumen.HardwareRayTracing.LightingMode"))
  (Variables|Default|SetLumenHardwareRayTracingLightingMode _returnvalue_4)
  (bind _returnvalue_5 (Development|GetConsoleVariableIntValue "r.HDR.Display.OutputDevice"))
  (Variables|Default|SetOriginalOutputDevice _returnvalue_5)
  (Development|ExecuteConsoleCommand "r.HDR.Display.OutputDevice 0" 0))

(event EventEndPlay
  (params (EndPlayReason :type EEndPlayReason%20Enum :default "Destroyed"))
  (Development|ExecuteConsoleCommand (Utilities|String|Append "r.HDR.Display.OutputDevice " (Utilities|String|ToString(Integer) (Variables|Default|GetOriginalOutputDevice))) 0))

(event EventTick
  (params (DeltaSeconds :type Float%20%28single-precision%29))
  (bind _returnvalue (Class|AximmetryFunctionLibrary|GetAximmetryLogical "B1 Data:B Mask" 121 false))
  (bind _returnvalue_2 (Class|AximmetryFunctionLibrary|GetAximmetryVector "Out Size" 0 "0, 0, 0"))
  (bind _returnvalue_3 (Class|AximmetryFunctionLibrary|GetAximmetryLogical "B1 Data:Virtuals" 120 false))
  (bind _returnvalue_4 (Class|AximmetryFunctionLibrary|GetAximmetryLogical "B1 Data:Tracked Cam Active" 10 false))
  (bind _returnvalue_5 (not _returnvalue_4))
  (|CallParentFunction DeltaSeconds)
  (if (< (Variables|Default|GetPrewarm) 5)
    (Math|Integer|IncrementInt (Variables|Default|GetPrewarm)
      (:%20%20
        (Rendering|SetActorHiddenInGame true)
        (bind _returnvalue_6 (Class|AximmetryFunctionLibrary|GetAximmetryVideo "B1 Texture" 110 false true "TA_Clamp" :!label _label))
        (bind _returnvalue_7 (Class|AximmetryFunctionLibrary|GetAximmetryVideo "B1 Refl Texture" 112 false true "TA_Clamp"))
        (bind _returnvalue_8 (Class|AximmetryFunctionLibrary|GetAximmetryVideo "B1 AO Texture" 111 true true "TA_Clamp"))
        (bind _returnvalue_9 (Class|AximmetryFunctionLibrary|GetAximmetryVideo "B1 Shadow Texture" 113 false false "TA_Clamp"))
        (CallFunction|UpdateBillboard _returnvalue (Variables|Default|GetB1%20Billboard) (Variables|Default|GetB1%20Reflection) (Variables|Default|GetB1%20Shadow) (Variables|Default|GetB1%20Depth) (Variables|Default|GetB1%20AO) (Variables|Default|GetB1%20Light%20Wrap%20Mask%20Capture) (Class|AximmetryFunctionLibrary|GetAximmetryLogical "B1 Data:Active" 100 false) _returnvalue_3 (Class|AximmetryFunctionLibrary|GetAximmetryLogical "B1 Data:Lit" 101 false) (Class|AximmetryFunctionLibrary|GetAximmetryLogical "B1 Data:Cast Shadow" 104 true) (Class|AximmetryFunctionLibrary|GetAximmetryLogical "B1 Data:Inverse Tonemap" 102 true) (Class|AximmetryFunctionLibrary|GetAximmetryTransformation "B1 Data:Transform" 106) (Class|AximmetryFunctionLibrary|GetAximmetryTransformation "B1 Data:Refl Transform" 108) (Class|AximmetryFunctionLibrary|GetAximmetryTransformation "B1 Data:AO Transform" 107) _returnvalue_6 _returnvalue_7 _returnvalue_8 _returnvalue_9 (Class|AximmetryFunctionLibrary|GetAximmetryScalar "B1 Data:Shadow Depth" 114 2e+01) (Class|AximmetryFunctionLibrary|GetAximmetryTransformation "B1 Data:Shadow Transform" 115) (Class|AximmetryFunctionLibrary|GetAximmetryLogical "B1 Data:Render To Depth" 0 true) (Class|AximmetryFunctionLibrary|GetAximmetryLogical "B1 Data:Alpha Correction" 0 false) (Class|AximmetryFunctionLibrary|GetAximmetryScalar "B1 Data:Ray Traced Reflection Intensity" 0 1.0))
        (bind _returnvalue_10 (Class|AximmetryFunctionLibrary|GetAximmetryVideo "B2 Texture" 210 false true "TA_Clamp"))
        (bind _returnvalue_11 (Class|AximmetryFunctionLibrary|GetAximmetryVideo "B2 Refl Texture" 212 false true "TA_Clamp"))
        (bind _returnvalue_12 (Class|AximmetryFunctionLibrary|GetAximmetryVideo "B2 AO Texture" 211 true true "TA_Clamp"))
        (bind _returnvalue_13 (Class|AximmetryFunctionLibrary|GetAximmetryVideo "B2 Shadow Texture" 213 false false "TA_Clamp"))
        (CallFunction|UpdateBillboard _returnvalue (Variables|Default|GetB2%20Billboard) (Variables|Default|GetB2%20Reflection) (Variables|Default|GetB2%20Shadow) (Variables|Default|GetB2%20Depth) (Variables|Default|GetB2%20AO) (Variables|Default|GetB2%20Light%20Wrap%20Mask%20Capture) (Class|AximmetryFunctionLibrary|GetAximmetryLogical "B2 Data:Active" 200 false) _returnvalue_3 (Class|AximmetryFunctionLibrary|GetAximmetryLogical "B2 Data:Lit" 201 false) (Class|AximmetryFunctionLibrary|GetAximmetryLogical "B2 Data:Cast Shadow" 204 true) (Class|AximmetryFunctionLibrary|GetAximmetryLogical "B2 Data:Inverse Tonemap" 202 true) (Class|AximmetryFunctionLibrary|GetAximmetryTransformation "B2 Data:Transform" 206) (Class|AximmetryFunctionLibrary|GetAximmetryTransformation "B2 Data:Refl Transform" 208) (Class|AximmetryFunctionLibrary|GetAximmetryTransformation "B2 Data:AO Transform" 207) _returnvalue_10 _returnvalue_11 _returnvalue_12 _returnvalue_13 (Class|AximmetryFunctionLibrary|GetAximmetryScalar "B2 Data:Shadow Depth" 214 2e+01) (Class|AximmetryFunctionLibrary|GetAximmetryTransformation "B2 Data:Shadow Transform" 215) (Class|AximmetryFunctionLibrary|GetAximmetryLogical "B2 Data:Render To Depth" 0 true) (Class|AximmetryFunctionLibrary|GetAximmetryLogical "B2 Data:Alpha Correction" 0 false) (Class|AximmetryFunctionLibrary|GetAximmetryScalar "B2 Data:Ray Traced Reflection Intensity" 0 1.0))
        (bind _returnvalue_14 (Class|AximmetryFunctionLibrary|GetAximmetryVideo "B3 Texture" 310 false true "TA_Clamp"))
        (bind _returnvalue_15 (Class|AximmetryFunctionLibrary|GetAximmetryVideo "B3 Refl Texture" 312 false true "TA_Clamp"))
        (bind _returnvalue_16 (Class|AximmetryFunctionLibrary|GetAximmetryVideo "B3 AO Texture" 311 true true "TA_Clamp"))
        (bind _returnvalue_17 (Class|AximmetryFunctionLibrary|GetAximmetryVideo "B3 Shadow Texture" 313 false false "TA_Clamp"))
        (CallFunction|UpdateBillboard _returnvalue (Variables|Default|GetB3%20Billboard) (Variables|Default|GetB3%20Reflection) (Variables|Default|GetB3%20Shadow) (Variables|Default|GetB3%20Depth) (Variables|Default|GetB3%20AO) (Variables|Default|GetB3%20Light%20Wrap%20Mask%20Capture) (Class|AximmetryFunctionLibrary|GetAximmetryLogical "B3 Data:Active" 300 false) _returnvalue_3 (Class|AximmetryFunctionLibrary|GetAximmetryLogical "B3 Data:Lit" 301 false) (Class|AximmetryFunctionLibrary|GetAximmetryLogical "B3 Data:Cast Shadow" 304 true) (Class|AximmetryFunctionLibrary|GetAximmetryLogical "B3 Data:Inverse Tonemap" 302 true) (Class|AximmetryFunctionLibrary|GetAximmetryTransformation "B3 Data:Transform" 306) (Class|AximmetryFunctionLibrary|GetAximmetryTransformation "B3 Data:Refl Transform" 308) (Class|AximmetryFunctionLibrary|GetAximmetryTransformation "B3 Data:AO Transform" 307) _returnvalue_14 _returnvalue_15 _returnvalue_16 _returnvalue_17 (Class|AximmetryFunctionLibrary|GetAximmetryScalar "B3 Data:Shadow Depth" 314 2e+01) (Class|AximmetryFunctionLibrary|GetAximmetryTransformation "B3 Data:Shadow Transform" 315) (Class|AximmetryFunctionLibrary|GetAximmetryLogical "B3 Data:Render To Depth" 0 true) (Class|AximmetryFunctionLibrary|GetAximmetryLogical "B3 Data:Alpha Correction" 0 false) (Class|AximmetryFunctionLibrary|GetAximmetryScalar "B3 Data:Ray Traced Reflection Intensity" 0 1.0))
        (bind _merged (Default|Tick (Variables|Default|GetMask%20Merger) (Variables|/Script/Engine.SceneCaptureComponent2D|GetTextureTarget (Variables|Default|GetB1%20Light%20Wrap%20Mask%20Capture)) (Variables|/Script/Engine.SceneCaptureComponent2D|GetTextureTarget (Variables|Default|GetB2%20Light%20Wrap%20Mask%20Capture)) (Variables|/Script/Engine.SceneCaptureComponent2D|GetTextureTarget (Variables|Default|GetB3%20Light%20Wrap%20Mask%20Capture))))
        (Class|AximmetryFunctionLibrary|SetAximmetryVideo "B Mask" 400 "NoColorSpace" false _merged)))
    (else
      (if (and (not (Variables|Default|GetActive)) _returnvalue_5)
        (Default|BeginPlay (Variables|Default|GetCamera) self))
      (bind _output_get (Variables|Default|SetActive _returnvalue_5))
      (Rendering|SetActorHiddenInGame (not _output_get))
      (if _output_get
        (if (!= (Math|Float|Round (.x (Class|AximmetryFunctionLibrary|GetAximmetryVector "Out Size" 0 "0, 0, 0"))) 0)
          (CallFunction|UpdateHDR (Class|AximmetryFunctionLibrary|GetAximmetryLogical "B1 Data:HDR" 0 false))
          (Default|Tick (Variables|Default|GetCamera) (Class|AximmetryFunctionLibrary|GetAximmetryScalar "Cam Horizontal FOV" 2 9e+01) (Class|AximmetryFunctionLibrary|GetAximmetryScalar "Cam Focus Distance" 3 2e+01) (/ (.x _returnvalue_2) (.y _returnvalue_2)) (Class|AximmetryFunctionLibrary|GetAximmetryTransformation "Cam Transform" 1))
          (goto _label))))))

(fn ConstructionScript
  (|CallParentFunction))

(fn UpdateBillboard
  (params (LightWrap :type Boolean) (BillboardComponent :type Billboard%20Object%20Reference) (ReflectionComponent :type Reflection%20Object%20Reference) (ShadowComponent :type Shadow%20Object%20Reference) (DepthComponent :type Depth%20Object%20Reference) (AOComponent :type AO%20Object%20Reference) (CaptureComponent :type Scene%20Capture%20Component%202D%20Object%20Reference) (Active :type Boolean) (Virtuals :type Boolean) (Lit :type Boolean) (CastShadow :type Boolean) (BypassTonemapper :type Boolean) (BillboardTransform :type Transform) (ReflectionTransform :type Transform) (AOTransform :type Transform) (BillboardTexture :type Texture%20Object%20Reference) (ReflectionTexture :type Texture%20Object%20Reference) (AOTexture :type Texture%20Object%20Reference) (ShadowTexture :type Texture%20Object%20Reference) (ShadowDepth :type Float%20%28double-precision%29) (ShadowTransform :type Transform) (EnableScreenSpaceReflections :type Boolean) (AlphaCorrection :type Boolean) (RayTracedReflectionIntensity :type Float%20%28single-precision%29))
  (bind _reflectionmethod (Variables|Default|GetReflectionMethod))
  (bind _raytracingshadows (Variables|Default|GetRayTracingShadows))
  (bind _lumenhardwareraytracinglightingmode (Variables|Default|GetLumenHardwareRayTracingLightingMode))
  (bind _reflectionmethod_2 (Variables|Default|GetReflectionMethod))
  (bind _reflectionmethod_3 (Variables|Default|GetReflectionMethod))
  (bind _hdr (Variables|Default|GetHDR))
  (bind _lumenhardwareraytracing (Variables|Default|GetLumenHardwareRayTracing))
  (bind _returnvalue (not _hdr))
  (bind _returnvalue_2 (== _lumenhardwareraytracinglightingmode 2))
  (bind _returnvalue_3 (== _reflectionmethod_2 3))
  (bind _returnvalue_4 (== _reflectionmethod_3 1))
  (bind _returnvalue_5 (Math|Boolean|ANDBoolean _returnvalue_4 _lumenhardwareraytracing _returnvalue_2))
  (bind _returnvalue_6 (and BypassTonemapper _returnvalue))
  (bind _returnvalue_7 (or _returnvalue_5 _returnvalue_3))
  (Utilities|FlowControl|Sequence
    (:then_0
      (if EnableScreenSpaceReflections
        (if CastShadow
          (if _raytracingshadows
            (switch int _reflectionmethod
              (:0
                (LocalVariables|SetReflectionComponentRendersPlanarReflections true)
                (LocalVariables|SetDepthComponentRendersScreenSpaceReflections false)
                (LocalVariables|SetDepthComponentRendersRayTracedReflections false)
                (LocalVariables|SetShadowComponentRendersRayTracedReflections false))
              (:1
                (LocalVariables|SetReflectionComponentRendersPlanarReflections false)
                (LocalVariables|SetDepthComponentRendersScreenSpaceReflections true)
                (LocalVariables|SetDepthComponentRendersRayTracedReflections false)
                (LocalVariables|SetShadowComponentRendersRayTracedReflections true))
              (:2
                (LocalVariables|SetReflectionComponentRendersPlanarReflections true)
                (LocalVariables|SetDepthComponentRendersScreenSpaceReflections true)
                (LocalVariables|SetDepthComponentRendersRayTracedReflections false)
                (LocalVariables|SetShadowComponentRendersRayTracedReflections false))
              (:3
                (LocalVariables|SetReflectionComponentRendersPlanarReflections false)
                (LocalVariables|SetDepthComponentRendersScreenSpaceReflections false)
                (LocalVariables|SetDepthComponentRendersRayTracedReflections false)
                (LocalVariables|SetShadowComponentRendersRayTracedReflections true)))
            (else
              (switch int _reflectionmethod :!label _label
                (:0
                  (LocalVariables|SetReflectionComponentRendersPlanarReflections true)
                  (LocalVariables|SetDepthComponentRendersScreenSpaceReflections false)
                  (LocalVariables|SetDepthComponentRendersRayTracedReflections false)
                  (LocalVariables|SetShadowComponentRendersRayTracedReflections false))
                (:1
                  (LocalVariables|SetReflectionComponentRendersPlanarReflections false)
                  (LocalVariables|SetDepthComponentRendersScreenSpaceReflections true)
                  (LocalVariables|SetDepthComponentRendersRayTracedReflections true)
                  (LocalVariables|SetShadowComponentRendersRayTracedReflections false))
                (:2
                  (LocalVariables|SetReflectionComponentRendersPlanarReflections true)
                  (LocalVariables|SetDepthComponentRendersScreenSpaceReflections true)
                  (LocalVariables|SetDepthComponentRendersRayTracedReflections false)
                  (LocalVariables|SetShadowComponentRendersRayTracedReflections false))
                (:3
                  (LocalVariables|SetReflectionComponentRendersPlanarReflections false)
                  (LocalVariables|SetDepthComponentRendersScreenSpaceReflections false)
                  (LocalVariables|SetDepthComponentRendersRayTracedReflections true)
                  (LocalVariables|SetShadowComponentRendersRayTracedReflections false)))))
          (elif _raytracingshadows
            (goto _label)
            (else
              (goto _label))))
        (elif CastShadow
          (if _raytracingshadows
            (switch int _reflectionmethod
              (:0
                (LocalVariables|SetReflectionComponentRendersPlanarReflections true)
                (LocalVariables|SetDepthComponentRendersScreenSpaceReflections false)
                (LocalVariables|SetDepthComponentRendersRayTracedReflections false)
                (LocalVariables|SetShadowComponentRendersRayTracedReflections false))
              (:1
                (LocalVariables|SetReflectionComponentRendersPlanarReflections false)
                (LocalVariables|SetDepthComponentRendersScreenSpaceReflections false)
                (LocalVariables|SetDepthComponentRendersRayTracedReflections false)
                (LocalVariables|SetShadowComponentRendersRayTracedReflections false))
              (:2
                (LocalVariables|SetReflectionComponentRendersPlanarReflections true)
                (LocalVariables|SetDepthComponentRendersScreenSpaceReflections false)
                (LocalVariables|SetDepthComponentRendersRayTracedReflections false)
                (LocalVariables|SetShadowComponentRendersRayTracedReflections false))
              (:3
                (LocalVariables|SetReflectionComponentRendersPlanarReflections false)
                (LocalVariables|SetDepthComponentRendersScreenSpaceReflections false)
                (LocalVariables|SetDepthComponentRendersRayTracedReflections false)
                (LocalVariables|SetShadowComponentRendersRayTracedReflections true)))
            (else
              (switch int _reflectionmethod :!label _label_2
                (:0
                  (LocalVariables|SetReflectionComponentRendersPlanarReflections true)
                  (LocalVariables|SetDepthComponentRendersScreenSpaceReflections false)
                  (LocalVariables|SetDepthComponentRendersRayTracedReflections false)
                  (LocalVariables|SetShadowComponentRendersRayTracedReflections false))
                (:1
                  (LocalVariables|SetReflectionComponentRendersPlanarReflections false)
                  (LocalVariables|SetDepthComponentRendersScreenSpaceReflections false)
                  (LocalVariables|SetDepthComponentRendersRayTracedReflections false)
                  (LocalVariables|SetShadowComponentRendersRayTracedReflections false))
                (:2
                  (LocalVariables|SetReflectionComponentRendersPlanarReflections true)
                  (LocalVariables|SetDepthComponentRendersScreenSpaceReflections false)
                  (LocalVariables|SetDepthComponentRendersRayTracedReflections false)
                  (LocalVariables|SetShadowComponentRendersRayTracedReflections false))
                (:3
                  (LocalVariables|SetReflectionComponentRendersPlanarReflections false)
                  (LocalVariables|SetDepthComponentRendersScreenSpaceReflections false)
                  (LocalVariables|SetDepthComponentRendersRayTracedReflections true)
                  (LocalVariables|SetShadowComponentRendersRayTracedReflections false)))))
          (elif _raytracingshadows
            (goto _label_2)
            (else
              (goto _label_2))))))
    (:then_1
      (Default|Tick BillboardComponent Active Virtuals Lit _returnvalue_6 BillboardTexture BillboardTransform AlphaCorrection)
      (Default|Tick ReflectionComponent (and Active (LocalVariables|GetReflectionComponentRendersPlanarReflections)) Lit _returnvalue_6 ReflectionTexture ReflectionTransform AlphaCorrection)
      (Default|Tick ShadowComponent (and Active (or CastShadow (LocalVariables|GetShadowComponentRendersRayTracedReflections))) ShadowTransform BillboardTexture ShadowTexture (Variables|Default|GetRayTracingShadows) ShadowDepth _returnvalue_6 Lit (select (and (LocalVariables|GetShadowComponentRendersRayTracedReflections) _returnvalue_7) RayTracedReflectionIntensity 0.0))
      (Default|Tick DepthComponent (and Active (or (LocalVariables|GetDepthComponentRendersScreenSpaceReflections) (LocalVariables|GetDepthComponentRendersRayTracedReflections))) BillboardTexture BillboardTransform _returnvalue_6 (LocalVariables|GetDepthComponentRendersRayTracedReflections) Lit (select (and _returnvalue_7 (LocalVariables|GetDepthComponentRendersRayTracedReflections)) RayTracedReflectionIntensity 0.0) (or (== (Variables|Default|GetReflectionMethod) 1) (== (Variables|Default|GetReflectionMethod) 2)))
      (Default|Tick AOComponent Active AOTexture AOTransform)
      (CallFunction|UpdateLightWrapCapture (and LightWrap Active) CaptureComponent BillboardTransform))))

(fn InitializeLightWrapCapture
  (params (CaptureComponent :type Scene%20Capture%20Component%202D%20Object%20Reference))
  (Variables|/Script/Engine.SceneCaptureComponent|SetCaptureSource CaptureComponent "SCS_FinalColorLDR")
  (Variables|/Script/Engine.SceneCaptureComponent|SetbCaptureEveryFrame CaptureComponent false)
  (Variables|/Script/Engine.SceneCaptureComponent|SetbCaptureOnMovement CaptureComponent false)
  (Variables|/Script/Engine.SceneCaptureComponent|SetbAlwaysPersistRenderingState CaptureComponent true)
  (Variables|/Script/Engine.SceneCaptureComponent2D|SetbEnableClipPlane CaptureComponent true)
  (Variables|/Script/Engine.SceneCaptureComponent2D|SetbForceTemporalJitter CaptureComponent true)
  (Variables|/Script/Engine.SceneCaptureComponent2D|SetbUseCustomProjectionMatrix CaptureComponent true)
  (Utilities|Struct|SetmembersinPostProcessSettings (Variables|/Script/Engine.SceneCaptureComponent2D|GetPostProcessSettings CaptureComponent) (Utilities|Struct|MakeWeightedBlendables (Utilities|Array|MakeArray (Utilities|Struct|MakeWeightedBlendable 1.0 "/Game/Aximmetry_VirtualCam_3-Bill/Materials/Alpha.Alpha") (Utilities|Struct|MakeWeightedBlendable 1.0 "/Game/Aximmetry_VirtualCam_3-Bill/Materials/Empty_Tonemapper.Empty_Tonemapper"))))
  (Variables|/Script/Engine.SceneCaptureComponent|SetPrimitiveRenderMode CaptureComponent "PRM_RenderScenePrimitives")
  (Class|SceneCaptureComponent|HideComponent CaptureComponent (Variables|Default|GetB1%20Reflection))
  (Class|SceneCaptureComponent|HideComponent CaptureComponent (Variables|Default|GetB2%20Reflection))
  (Class|SceneCaptureComponent|HideComponent CaptureComponent (Variables|Default|GetB3%20Reflection)))

(fn UpdateLightWrapCapture
  (params (Active :type Boolean) (CaptureComponent :type Scene%20Capture%20Component%202D%20Object%20Reference) (BillboardTransform :type Transform%20%28by%20ref%29))
  (bind _returnvalue (Math|Transform|TransformDirection BillboardTransform "0,0.000000,1.000000"))
  (bind _returnvalue_2 (Class|AximmetryFunctionLibrary|GetAximmetryVector "Out Size" 0 "0, 0, 0"))
  (bind _returnvalue_3 (Math|Float|Round (.x _returnvalue_2)))
  (bind _returnvalue_4 (Math|Float|Round (.y _returnvalue_2)))
  (if Active
    (if (Utilities|IsValid (Variables|/Script/Engine.SceneCaptureComponent2D|GetTextureTarget CaptureComponent))
      (if (or (!= (Variables|/Script/Engine.TextureRenderTarget2D|GetSizeX (Variables|/Script/Engine.SceneCaptureComponent2D|GetTextureTarget CaptureComponent)) _returnvalue_3) (!= (Variables|/Script/Engine.TextureRenderTarget2D|GetSizeY (Variables|/Script/Engine.SceneCaptureComponent2D|GetTextureTarget CaptureComponent)) _returnvalue_4))
        (bind _returnvalue_5 (Rendering|CreateRenderTarget2D _returnvalue_3 _returnvalue_4 "RTF_R16f" :!label _label))
        (Variables|/Script/Engine.SceneCaptureComponent2D|SetTextureTarget CaptureComponent _returnvalue_5))
      (else
        (goto _label)))
    (bind _desiredview (Class|CameraComponent|GetCameraView (Variables|Default|GetCamera) 0.0))
    (Variables|/Script/Engine.SceneCaptureComponent2D|SetCustomProjectionMatrix CaptureComponent (.ProjectionMatrix (Class|GameplayStatics|GetViewProjectionMatrix _desiredview)))
    (Variables|/Script/Engine.SceneCaptureComponent2D|SetClipPlaneBase CaptureComponent (+ (Math|Transform|TransformLocation BillboardTransform "0, 0,1.000000") _returnvalue))
    (Variables|/Script/Engine.SceneCaptureComponent2D|SetClipPlaneNormal CaptureComponent _returnvalue)
    (Rendering|SceneCapture|CaptureScene CaptureComponent :!class /Script/Engine.SceneCaptureComponent2D)
    (else
      (Variables|/Script/Engine.SceneCaptureComponent2D|SetTextureTarget CaptureComponent 0))))

(fn UpdateHDR
  (params (HDR :type Boolean))
  (bind _returnvalue (Utilities|String|MakeLiteralString "Error: Wrong Frame Buffer Pixel Format. HDR rendering will not work correctly.  
Please set Frame Buffer Pixel Format to \"Float RGBA\" in the Unreal Project Settings."))
  (bind _camera (Variables|Default|GetCamera))
  (bind _postprocesssettings (Variables|/Script/Engine.CameraComponent|GetPostProcessSettings _camera))
  (bind _weightedblendables (Utilities|Struct|BreakPostProcessSettings _postprocesssettings))
  (bind _array (Utilities|Struct|BreakWeightedBlendables _weightedblendables))
  (bind _output (Utilities|Array|Get(acopy) _array))
  (if (!= HDR (Variables|Default|GetHDR))
    (bind _output_get (Variables|Default|SetHDR HDR))
    (if _output_get
      (Development|ExecuteConsoleCommand "r.HDR.Display.OutputDevice 7" 0)
      (Utilities|Struct|SetmembersinWeightedBlendable _output 1.0)
      (bind _returnvalue_2 (Development|GetConsoleVariableIntValue "r.DefaultBackBufferPixelFormat"))
      (if (!= _returnvalue_2 3)
        (Development|PrintString _returnvalue true false "(R=1.000000,G=0.000000,B=0.000000,A=1.000000)" 999999.0 "AximmetryHDRPixelFormatError")
        (Class|AximmetryFunctionLibrary|Log _returnvalue "Error"))
      (else
        (Development|ExecuteConsoleCommand "r.HDR.Display.OutputDevice 0" 0)
        (Utilities|Struct|SetmembersinWeightedBlendable _output 0.0)
        (Development|PrintString "" true false "(R=1.000000,G=0.000000,B=0.000000,A=1.000000)" 0.0 "AximmetryHDRPixelFormatError") ; Clear onscreen warning
      ))))